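; VRPlayerController is a Leap Motion player controller that adjusts control rotation when head-mounted display mode changes.
; Tick compares the HMD enabled state against a stored flag and fires enter or exit events on a change.
; Entering zeroes pitch and roll while keeping yaw; exiting does nothing.
; An uncalled helper, SetControlRotationFromHMD, copies HMD pitch and roll into control rotation with zero yaw.
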(event `EnteredHMDMode`
  (`self.ZeroControlRotation`))

(event `ExitedHMDMode`)

(event `self.ReceiveTick`
  (params (DeltaSeconds :type "Float (single-precision)"))
  (bind _returnvalue (`HeadMountedDisplayFunctionLibrary.IsHeadMountedDisplayEnabled`))
  ;[1 1 1] Check For HMD state change, and emit events
  (if (!= _returnvalue (`self.OldHMDEnabled`))
    (`|ExecutionSequence`
      (:`then_0`
        (if _returnvalue
          (`self.EnteredHMDMode`)
          (else
            (`self.ExitedHMDMode`))))
      (:`then_1`
        (set `self.OldHMDEnabled` _returnvalue)))))

(fn `SetControlRotationFromHMD`
  (`self.SetControlRotation` (`KismetMathLibrary.MakeRot` (.pitch (`HeadMountedDisplayFunctionLibrary.GetOrientationAndPosition`)) 0.0 (.roll (`HeadMountedDisplayFunctionLibrary.GetOrientationAndPosition`)))))

(fn `UserConstructionScript`)

(fn `ZeroControlRotation`
  (`self.SetControlRotation` (`KismetMathLibrary.MakeRot` 0.0 (.yaw (`self.GetControlRotation`)))))