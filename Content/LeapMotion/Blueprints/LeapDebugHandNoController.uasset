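; Leap Motion debug Blueprint with helpers that visualize tracked hand and finger data as debug spheres around the actor.
; DebugFinger marks the four bone centers of a finger and DebugHand marks the wrist and elbow, both through DebugSphereAtActor.
; That helper rotates each point by the negated device yaw combined with actor rotation, then scales it and offsets it by actor location.
; No graph shown calls DebugFinger or DebugHand.
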(fn ConstructionScript)

(fn DebugSphereatActor
  (params (Location :type Vector :default "0, 0, 0") (Scale :type Float%20%28single-precision%29) (Radius :type Float%20%28single-precision%29))
  (Rendering|Debug|DrawDebugSphere (+ (* (Math|Vector|RotateVector Location (Math|Rotator|CombineRotators (Class|KismetMathLibrary|MakeRot 0.0 (* (.Yaw (Class|KismetMathLibrary|BreakRot (.DeviceRotation (Class|HeadMountedDisplayFunctionLibrary|GetOrientationandPosition)))) -1.0) 0.0) (Transformation|GetActorRotation))) Scale) (Transformation|GetActorLocation)) Radius 12 "(R=0.000000,G=0.000000,B=0.000000,A=1.000000)" 0.0))

(fn DebugFinger
  (params (Finger :type Finger%20Object%20Reference) (Scale :type Float%20%28single-precision%29))
  (CallFunction|DebugSphereatActor (Variables|/Script/LeapMotion.Bone|GetCenter (Variables|/Script/LeapMotion.Finger|GetDistal Finger)) Scale Scale)
  (CallFunction|DebugSphereatActor (Variables|/Script/LeapMotion.Bone|GetCenter (Variables|/Script/LeapMotion.Finger|GetIntermediate Finger)) Scale Scale)
  (CallFunction|DebugSphereatActor (Variables|/Script/LeapMotion.Bone|GetCenter (Variables|/Script/LeapMotion.Finger|GetProximal Finger)) Scale Scale)
  (CallFunction|DebugSphereatActor (Variables|/Script/LeapMotion.Bone|GetCenter (Variables|/Script/LeapMotion.Finger|GetMetacarpal Finger)) Scale Scale))

(fn DebugHand
  (params (Hand :type Hand%20Object%20Reference) (Scale :type Float%20%28single-precision%29))
  (bind _arm (Variables|/Script/LeapMotion.Hand|GetArm Hand))
  (LocalVariables|SetElbowRadius 4.0)
  (LocalVariables|SetWrist%20Radius 2.0)
  (CallFunction|DebugSphereatActor (Variables|/Script/LeapMotion.Arm|GetWristPosition _arm) Scale (LocalVariables|GetWrist%20Radius))
  (CallFunction|DebugSphereatActor (Variables|/Script/LeapMotion.Arm|GetElbowPosition _arm) Scale (LocalVariables|GetElbowRadius)))